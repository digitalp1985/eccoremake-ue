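; Player is a flipbook-sprite pawn that swims left and right.
; BeginPlay adds two Enhanced Input mapping contexts to the BP_PlayerController and starts it facing right.
; IA_Default drives movement along the forward vector, with the axis sign choosing the swim flipbook and FacingRight, which selects the idle flipbook on release.
; IA_Default2 forwards X and Y to InputHandler, a stub that only returns zero.
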(event `self.ReceiveBeginPlay`
  (bind _asbp_player_controller (cast `/Game/Player/Blueprints/BP_PlayerController` (`self.GetController`)))
  (bind _returnvalue (pcsubsystem `EnhancedInputLocalPlayerSubsystem` _asbp_player_controller))
  (`EnhancedInputSubsystemInterface.AddMappingContext` _returnvalue "/Game/Player/Blueprints/IMC_Default.IMC_Default" 0 (struct))
  (set `self.Facing_Right` true)
  (`EnhancedInputSubsystemInterface.AddMappingContext` _returnvalue "/Game/Player/Blueprints/IMC_Def2.IMC_Def2" 0 (struct)))

(event `EnhancedInput|/Game/Player/Blueprints/IA_Default`
  (params (ActionValue :type "Float (double-precision)") (ElapsedSeconds :type "Float (double-precision)") (TriggeredSeconds :type "Float (double-precision)") (InputAction :type "InputAction Object Reference" :default "/Game/Player/Blueprints/IA_Default.IA_Default"))
  (:`Triggered`
    (`self.AddMovementInput` (`self.GetActorForwardVector`) ActionValue)
    (if (> ActionValue 0.0)
      (`PaperFlipbookComponent.SetFlipbook` (`self.Sprite`) "/Game/Player/Sprites/FinishedSprites/Swim/SwimRight/Swim_Right.Swim_Right")
      (set `self.Facing_Right` true)
      (else
        (`PaperFlipbookComponent.SetFlipbook` (`self.Sprite`) "/Game/Player/Sprites/FinishedSprites/Swim/SwimLeft/Swim_Left.Swim_Left")
        (set `self.Facing_Right` false))))
  (:`Completed`
    (if (`self.Facing_Right`)
      (`PaperFlipbookComponent.SetFlipbook` (`self.Sprite`) "/Game/Player/Sprites/FinishedSprites/Idle/Idle_Right.Idle_Right")
      (else
        (`PaperFlipbookComponent.SetFlipbook` (`self.Sprite`) "/Game/Player/Sprites/FinishedSprites/Idle/Idle_Left.Idle_Left")))))

(event `EnhancedInput|/Game/Player/Blueprints/IA_Default2`
  (params (ActionValue :type "Vector2D Structure") (ElapsedSeconds :type "Float (double-precision)") (TriggeredSeconds :type "Float (double-precision)") (InputAction :type "InputAction Object Reference" :default "/Game/Player/Blueprints/IA_Default2.IA_Default2"))
  (:`Triggered`
    (`self.InputHandler` ActionValue_X ActionValue_Y)))

(fn `InputHandler`
  (params (Xinput :type "Float (double-precision)") (YInput :type "Float (double-precision)"))
  (returns (Direction :type Integer))
  (return 0))

(fn `UserConstructionScript`)